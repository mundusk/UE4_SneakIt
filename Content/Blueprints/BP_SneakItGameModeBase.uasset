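; Game mode Blueprint for SneakIt, a relic-stealing game, that manages the HUD and game-over screens.
; BeginPlay shows WBP_HUD with total and stolen relic counts.
; Each successful theft creates a fresh HUD with the new count, removing only the BeginPlay instance, so later HUDs stack.
; Completing the relic theft adds WBP_GameOver, passing it the stolen-relic result.
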(event EventOnCompletedStealingRelics
  (params (bRelicsStealSuccess :type Boolean))
  (Utilities|FlowControl|Sequence
    (:then_0
      (bind _returnvalue (UserInterface|CreateWidget "/Game/UI/WBP_GameOver.WBP_GameOver_C" 0 bRelicsStealSuccess))
      (UserInterface|Viewport|AddtoViewport _returnvalue 0))))

(event EventOnRelicSuccessfullyStolen
  (params (NumberOfStolenRelics :type Integer))
  (Widget|RemovefromParent (stale EventBeginPlay _returnvalue))
  (bind _returnvalue (UserInterface|CreateWidget "/Game/UI/WBP_HUD.WBP_HUD_C" 0 (Variables|Default|GetTotalRelics) NumberOfStolenRelics))
  (UserInterface|Viewport|AddtoViewport _returnvalue 0))

(event EventBeginPlay
  (Utilities|FlowControl|Sequence
    (:then_0
      (bind _returnvalue (UserInterface|CreateWidget "/Game/UI/WBP_HUD.WBP_HUD_C" 0 (Variables|Default|GetTotalRelics) (Variables|Default|GetRelicsStolen)))
      (UserInterface|Viewport|AddtoViewport _returnvalue 0))))

(fn ConstructionScript)